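; BP_VolumetricFog is a box-bounded volumetric fog actor with configurable shape, noise, color, shadow and height falloff.
; Construction creates fog and interaction material instances plus render targets, passes the fog material to Niagara and runs a grid-pixel-size console command.
; Orthographic captures of listed actors, from the volume's top and bottom, supply height and interaction textures to those materials.
; Tick repositions and re-captures only the height view each frame.
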(event `self.ReceiveTick`
  (params (DeltaSeconds :type "Float (single-precision)"))
  (`self.HeightCaptureSetup`))

(fn `CaptureHeight`
  (`SceneCaptureComponent2D.CaptureScene` (`self.HeightCapture`))
  (return))

(fn `HeightCaptureSetup`
  (bind (_returnvalue_x _returnvalue_y _returnvalue_z) (`KismetMathLibrary.BreakVector` (`self.K2_GetActorLocation`)))
  (bind _heightcapture (`self.HeightCapture`))
  (bind (_volumesize_x _volumesize_y _volumesize_z) (`KismetMathLibrary.BreakVector` (`self.VolumeSize`)))
  (bind (_volumesize_x_2 _volumesize_y_2 _volumesize_z_2) (`KismetMathLibrary.BreakVector` (`self.VolumeSize`)))
  ;[1 1 1] Height capture settings
  (`SceneComponent.K2_SetWorldLocationAndRotation` _heightcapture (`KismetMathLibrary.MakeVector` _returnvalue_x _returnvalue_y (+ _returnvalue_z (/ _volumesize_z_2 2.0))) (struct :`Pitch` -90.0 :`Roll` -90.0) false false)
  (set `SceneCaptureComponent2D.OrthoWidth` (`KismetMathLibrary.FMax` (`KismetMathLibrary.FMax` _volumesize_x _volumesize_y) _volumesize_z) _heightcapture)
  (set `SceneCaptureComponent2D.TextureTarget` (`self.FogHeightCaptureRT`) _heightcapture)
  (set `SceneCaptureComponent.ShowOnlyActors` (`self.HeightActors`) _heightcapture)
  (`self.CaptureHeight`))

(fn `InteractionCaptureSetup`
  (bind (_returnvalue_x _returnvalue_y _returnvalue_z) (`KismetMathLibrary.BreakVector` (`self.K2_GetActorLocation`)))
  (bind _interactioncapture (`self.InteractionCapture`))
  (bind (_volumesize_x _volumesize_y _volumesize_z) (`KismetMathLibrary.BreakVector` (`self.VolumeSize`)))
  (bind (_volumesize_x_2 _volumesize_y_2 _volumesize_z_2) (`KismetMathLibrary.BreakVector` (`self.VolumeSize`)))
  ;[1 1 1] Interactive Capture Settings
  (`SceneComponent.K2_SetWorldLocationAndRotation` _interactioncapture (`KismetMathLibrary.MakeVector` _returnvalue_x _returnvalue_y (- _returnvalue_z (/ _volumesize_z_2 2.0))) (struct :`Pitch` 90.0 :`Yaw` 90.0 :`Roll` 180.0) false false)
  (set `SceneCaptureComponent2D.OrthoWidth` (`KismetMathLibrary.FMax` (`KismetMathLibrary.FMax` _volumesize_x _volumesize_y) _volumesize_z) _interactioncapture)
  (set `SceneCaptureComponent2D.TextureTarget` (`self.FogInteractionCaptureRT`) _interactioncapture)
  (set `SceneCaptureComponent.ShowOnlyActors` (`self.InteractionActors`) _interactioncapture)
  (return))

(fn `SetFogMID_Variables`
  (bind _fogmid (`self.FogMID`))
  ;[1 1 1] Base Shape
  (`MaterialInstanceDynamic.SetVectorParameterValue` _fogmid "ShapeType" (select `/Game/VolumetricFog/BP/Enum/E_FogShapeType` (`self.ShapeType`) :`NewEnumerator0` (struct :`B` 1.0) :`NewEnumerator1` (struct :`A` 1.0) :`NewEnumerator2` (struct :`G` 1.0) :`NewEnumerator3` (struct :`R` 1.0) :!type "LinearColor Structure"))
  (`MaterialInstanceDynamic.SetVectorParameterValue` _fogmid "VolumeSize" (`KismetMathLibrary.Conv_VectorToLinearColor` (`self.VolumeSize`)))
  (`MaterialInstanceDynamic.SetTextureParameterValue` _fogmid "Texture2D" (`self.Texture2D`))
  (`MaterialInstanceDynamic.SetTextureParameterValue` _fogmid "VolumeTexture" (`self.VolumeTexture`))
  (`MaterialInstanceDynamic.SetScalarParameterValue` _fogmid "EdgeFalloff" (`self.EdgeFalloff`))
  (`MaterialInstanceDynamic.SetScalarParameterValue` _fogmid "FlowSpeed" (`self.BaseSpeed`))
  ;[1 1 1] Height Falloff
  (`MaterialInstanceDynamic.SetScalarParameterValue` _fogmid "GlobalHeightFalloff" (`self.GlobalHeightFalloff`))
  (`MaterialInstanceDynamic.SetTextureParameterValue` _fogmid "HeightRT" (`self.FogHeightCaptureRT`))
  (`MaterialInstanceDynamic.SetVectorParameterValue` _fogmid "HeightMethod" (select `/Game/VolumetricFog/BP/Enum/E_FogHeightMethod` (`self.HeightMethod`) :`NewEnumerator4` (struct :`R` 1.0) :`NewEnumerator5` (struct :`G` 1.0) :`NewEnumerator6` (struct :`B` 1.0) :`NewEnumerator7` (struct :`A` 1.0) :!type "LinearColor Structure"))
  (`MaterialInstanceDynamic.SetScalarParameterValue` _fogmid "GlobalHeightPower" (`self.GlobalHeightPower`))
  ;[1 1 1] Fog Settings
  (`MaterialInstanceDynamic.SetScalarParameterValue` _fogmid "GlobalExtinction" (`self.GlobalExtinction`))
  (`MaterialInstanceDynamic.SetVectorParameterValue` _fogmid "FogColor" (`self.FogColor`))
  (`MaterialInstanceDynamic.SetVectorParameterValue` _fogmid "ExtinctionColor" (`self.ExtinctionColor`))
  (`MaterialInstanceDynamic.SetVectorParameterValue` _fogmid "ShadowColor" (`self.ShadowColor`))
  (`MaterialInstanceDynamic.SetScalarParameterValue` _fogmid "ShadowTraceDist" (`self.ShadowTraceDist`))
  (`MaterialInstanceDynamic.SetScalarParameterValue` _fogmid "ShadowFalloffDist" (`self.ShadowFalloffDist`))
  (`MaterialInstanceDynamic.SetScalarParameterValue` _fogmid "FogColorIntensity" (`self.FogColorIntensity`))
  (`MaterialInstanceDynamic.SetScalarParameterValue` _fogmid "ShadowDensity" (`self.ShadowDensity`))
  (`MaterialInstanceDynamic.SetScalarParameterValue` _fogmid "NoiseScale" (`self.NoiseScale`))
  (`MaterialInstanceDynamic.SetScalarParameterValue` _fogmid "NoisePower" (`self.NoisePower`))
  ;[1 1 1] Noise02 setting
  (`MaterialInstanceDynamic.SetScalarParameterValue` _fogmid "Noise02 Scale" (`self.Noise02 Scale`))
  (`MaterialInstanceDynamic.SetScalarParameterValue` _fogmid "Noise02  Speed" (`self.Noise02  Speed`))
  (`MaterialInstanceDynamic.SetTextureParameterValue` _fogmid "Noise02 Tex" (`self.Noise02 VolumeTexture`))
  ;[1 1 1] Bump Setting
  (`MaterialInstanceDynamic.SetScalarParameterValue` _fogmid "Bump Scale" (`self.Bump Scale`))
  (`MaterialInstanceDynamic.SetVectorParameterValue` _fogmid "Bump Speed" (`self.Bump Speed`))
  (`MaterialInstanceDynamic.SetScalarParameterValue` _fogmid "Bump Power" (`self.Bump Power`))
  (`MaterialInstanceDynamic.SetTextureParameterValue` _fogmid "Bump Tex" (`self.Bump Volume Texture`))
  (return))

(fn `SetInteractionMID_Variables`
  (bind _interactionmid (`self.InteractionMID`))
  ;[1 1 1] Material instance interaction variable settings
  (`MaterialInstanceDynamic.SetTextureParameterValue` _interactionmid "InteractionCaptureRT" (`self.FogInteractionCaptureRT`))
  (`MaterialInstanceDynamic.SetTextureParameterValue` _interactionmid "HeightCaptureRT" (`self.FogHeightCaptureRT`))
  (`MaterialInstanceDynamic.SetScalarParameterValue` _interactionmid "FogHeight" (`self.GlobalHeightFalloff`))
  (return))

(fn `SetNiagaraVariables`
  (bind _ns_fogwrite (`self.NS_FogWrite`))
  (bind (_volumesize_x _volumesize_y _volumesize_z) (`KismetMathLibrary.BreakVector` (`self.VolumeSize`)))
  ;[1 1 1] Niagara particle variable settings
  (`NiagaraComponent.SetVariableMaterial` _ns_fogwrite "FogMID" (`self.FogMID`))
  (`NiagaraComponent.SetVariableFloat` _ns_fogwrite "VolumeSizeMax" (* (`KismetMathLibrary.FMax` (`KismetMathLibrary.FMax` _volumesize_x _volumesize_y) _volumesize_z) 2.0))
  (return))

(fn `UserConstructionScript`
  ;[1 1 1] Material instance settings and Render Target 2D settings
  (bind _returnvalue (`KismetMaterialLibrary.CreateDynamicMaterialInstance` "/Game/VolumetricFog/Mat/Ins/M_Fog_Inst.M_Fog_Inst"))
  (set `self.FogMID` _returnvalue)
  (bind _returnvalue_2 (`KismetRenderingLibrary.CreateRenderTarget2D` 256 256 "RTF_R32f"))
  (set `self.FogHeightCaptureRT` _returnvalue_2)
  (bind _returnvalue_3 (`KismetMaterialLibrary.CreateDynamicMaterialInstance` "/Game/VolumetricFog/Mat/Func/M_DrawInteraction.M_DrawInteraction"))
  (set `self.InteractionMID` _returnvalue_3)
  (bind _returnvalue_4 (`KismetRenderingLibrary.CreateRenderTarget2D` 256 256 "RTF_R32f"))
  (set `self.FogInteractionCaptureRT` _returnvalue_4)
  (bind _returnvalue_5 (`KismetRenderingLibrary.CreateRenderTarget2D` 256 256 "RTF_R16f"))
  (set `self.FogInteractionRT` _returnvalue_5)
  ;[1 1 1] Set the volume fog box range
  (`BoxComponent.SetBoxExtent` (`self.DebugBox`) (/ (`self.VolumeSize`) 2.0) true)
  ;[1 1 1] Function Settings
  (`self.SetNiagaraVariables`)
  (`self.SetFogMID_Variables`)
  (`self.HeightCaptureSetup`)
  (`self.InteractionCaptureSetup`)
  (`self.SetInteractionMID_Variables`)
  (`self.VolumetrticFog PixelSize`))

(fn `VolumetrticFog PixelSize`
  ;[1 1 1] r.VolumetricFog.GridPixelSize
  (for (_array_element _array_index) (`|MakeArray` (`self.Cmd Name`))
    (bind _returnvalue (`KismetStringLibrary.Concat_StrStr` _array_element " " (`KismetStringLibrary.Conv_DoubleToString` (`|GetArrayItem` (`|MakeArray` (`self.Fog Pixel Size`)) _array_index))))
    (`KismetSystemLibrary.PrintString` _returnvalue)
    (`KismetSystemLibrary.ExecuteConsoleCommand` _returnvalue null)
    (return)))