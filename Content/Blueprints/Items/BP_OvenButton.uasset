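; BP_OvenButton is an oven's on/off button, toggling cooking for the items in its referenced oven.
; CookEvent flip-flops between OpenOven and CloseOven, which move the button, set the oven's Clicked flag and assign or clear each item's oven reference.
; OpenOven also calls MultipleCook once per item.
; A delayed Tick check calls CloseOven whenever the oven is empty, without resetting the flip-flop.
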(event `self.ReceiveTick`
  (params (DeltaSeconds :type "Float (single-precision)"))
  (`KismetSystemLibrary.Delay` 2.0)
  (bind _ovenref (`self.OvenRef`)
    (:`then`
      (if (`KismetArrayLibrary.Array_IsEmpty` (`/Game/FirstPerson/Blueprints/Items/BP_Ovenn.Items` _ovenref))
        (`self.CloseOven`)))
    (:`else`)))

(event `Cook Event`
  (`self.OvenRef`
    (:`then`
      (`/Engine/EditorBlueprintResources/StandardMacros.FlipFlop`
        (:`A`
          (`self.OpenOven`))
        (:`B`
          (`self.CloseOven`))))
    (:`else`)))

(fn `CloseOven`
  (`SceneComponent.K2_SetRelativeLocation` (`self.Button`) (0.0 0.0 0.0) false false)
  (set `/Game/FirstPerson/Blueprints/Items/BP_Ovenn.Clicked?` false (`self.OvenRef`))
  (for _array_element (`/Game/FirstPerson/Blueprints/Items/BP_Ovenn.Items` (`self.OvenRef`))
    (set `/Game/FirstPerson/Blueprints/Items/BP_BaseItem.OvenRef` null _array_element)))

(fn `OpenOven`
  (set `/Game/FirstPerson/Blueprints/Items/BP_Ovenn.Clicked?` true (`self.OvenRef`))
  (`SceneComponent.K2_SetRelativeLocation` (`self.Button`) (0.0 5.0 0.0) false false)
  (for _array_element (`/Game/FirstPerson/Blueprints/Items/BP_Ovenn.Items` (`self.OvenRef`))
    (set `/Game/FirstPerson/Blueprints/Items/BP_BaseItem.OvenRef` (`self.OvenRef`) _array_element)
    (`/Game/FirstPerson/Blueprints/Items/BP_Ovenn.MultipleCook` (`self.OvenRef`))))

(fn `UserConstructionScript`)