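; BP_Ovenn is an oven actor that cooks BP_BaseItem food placed on its five slots.
; Each slot's overlap records itself on items in a given state and ignores a trace channel to mark it occupied.
; When clicked, MultipleCook starts each item's Cooking timer by function name and schedules a bell sound.
; The older Cook event remains, and the self-recursive overcook sound check is disconnected from MultipleCook.
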(event `PlayCookSound`
  (params (Delay :type "Float (double-precision)"))
  (`KismetSystemLibrary.Delay` Delay)
  (`GameplayStatics.PlaySoundAtLocation` "/Game/SFX/BellSFX.BellSFX" (`self.K2_GetActorLocation`) (struct) 1.0 1.0 0.15 null null null null)
  (`KismetSystemLibrary.PrintString` "arrived"))

(event `PalyOverCookSound`
  (`GameplayStatics.PlaySoundAtLocation` "/Game/SFX/overcookSfx.overcookSfx" (`self.K2_GetActorLocation`) (struct) 1.0 1.0 0.2 null null null null)
  (`KismetSystemLibrary.PrintString` "pırt"))

(event `Cook`
  (params (Item :type "/Game/FirstPerson/Blueprints/Items/BP_BaseItem Object Reference") (Location :type "Vector Structure"))
  ;[1 1 1] Old CookingCode
  (if (`self.Clicked?`)
    (for _array_element (`|MakeArray` Item)
      (set `self.ItemRef` _array_element)
      (set `/Game/FirstPerson/Blueprints/Items/BP_BaseItem.ItemState` "NewEnumerator2" (`self.ItemRef`))
      (if (`|EnumEquality` (`/Game/FirstPerson/Blueprints/Items/BP_BaseItem.ItemState` (`self.ItemRef`)) "NewEnumerator2")
        (if (`|EnumEquality` (`/Game/FirstPerson/Blueprints/Items/BP_BaseItem.CookState` (`self.ItemRef`)) "NewEnumerator0")
          (bind _returnvalue (`KismetSystemLibrary.K2_SetTimer` (`self.ItemRef`) "Cooking" 2.0))
          (elif (`|EnumEquality` (`/Game/FirstPerson/Blueprints/Items/BP_BaseItem.CookState` (`self.ItemRef`)) "NewEnumerator2")
            (`KismetSystemLibrary.K2_SetTimer` (`self.ItemRef`) "OverCooking" 2.0)))
        (else
          (`KismetSystemLibrary.K2_ClearAndInvalidateTimerHandle` _returnvalue))))))

(event `self.SpaceOne.OnComponentBeginOverlap`
  (params (OverlappedComponent :type "PrimitiveComponent Object Reference") (OtherActor :type "Actor Object Reference") (OtherComp :type "PrimitiveComponent Object Reference") (OtherBodyIndex :type Integer) (bFromSweep :type Boolean) (SweepResult :type "HitResult Structure (by ref)"))
  (bind _asbp_base_item (cast `/Game/FirstPerson/Blueprints/Items/BP_BaseItem` OtherActor))
  (if (`|EnumEquality` (`/Game/FirstPerson/Blueprints/Items/BP_BaseItem.ItemState` _asbp_base_item) "NewEnumerator2")
    (`PrimitiveComponent.SetCollisionResponseToChannel` (`self.SpaceOne`) "ECC_GameTraceChannel3" "ECR_Ignore")
    (set `/Game/FirstPerson/Blueprints/Items/BP_BaseItem.SpaceBoxRef` (`self.SpaceOne`) _asbp_base_item)))

(event `self.SpaceTwo.OnComponentBeginOverlap`
  (params (OverlappedComponent :type "PrimitiveComponent Object Reference") (OtherActor :type "Actor Object Reference") (OtherComp :type "PrimitiveComponent Object Reference") (OtherBodyIndex :type Integer) (bFromSweep :type Boolean) (SweepResult :type "HitResult Structure (by ref)"))
  (bind _asbp_base_item (cast `/Game/FirstPerson/Blueprints/Items/BP_BaseItem` OtherActor))
  (if (`|EnumEquality` (`/Game/FirstPerson/Blueprints/Items/BP_BaseItem.ItemState` _asbp_base_item) "NewEnumerator2")
    (`PrimitiveComponent.SetCollisionResponseToChannel` (`self.SpaceTwo`) "ECC_GameTraceChannel3" "ECR_Ignore")
    (set `/Game/FirstPerson/Blueprints/Items/BP_BaseItem.SpaceBoxRef` (`self.SpaceTwo`) _asbp_base_item)
    (`KismetSystemLibrary.PrintString` "2")))

(event `self.SpaceThree.OnComponentBeginOverlap`
  (params (OverlappedComponent :type "PrimitiveComponent Object Reference") (OtherActor :type "Actor Object Reference") (OtherComp :type "PrimitiveComponent Object Reference") (OtherBodyIndex :type Integer) (bFromSweep :type Boolean) (SweepResult :type "HitResult Structure (by ref)"))
  (bind _asbp_base_item (cast `/Game/FirstPerson/Blueprints/Items/BP_BaseItem` OtherActor))
  (if (`|EnumEquality` (`/Game/FirstPerson/Blueprints/Items/BP_BaseItem.ItemState` _asbp_base_item) "NewEnumerator2")
    (`PrimitiveComponent.SetCollisionResponseToChannel` (`self.SpaceThree`) "ECC_GameTraceChannel3" "ECR_Ignore")
    (set `/Game/FirstPerson/Blueprints/Items/BP_BaseItem.SpaceBoxRef` (`self.SpaceThree`) _asbp_base_item)
    (`KismetSystemLibrary.PrintString` "3")))

(event `self.SpaceFour.OnComponentBeginOverlap`
  (params (OverlappedComponent :type "PrimitiveComponent Object Reference") (OtherActor :type "Actor Object Reference") (OtherComp :type "PrimitiveComponent Object Reference") (OtherBodyIndex :type Integer) (bFromSweep :type Boolean) (SweepResult :type "HitResult Structure (by ref)"))
  (bind _asbp_base_item (cast `/Game/FirstPerson/Blueprints/Items/BP_BaseItem` OtherActor))
  (if (`|EnumEquality` (`/Game/FirstPerson/Blueprints/Items/BP_BaseItem.ItemState` _asbp_base_item) "NewEnumerator2")
    (`PrimitiveComponent.SetCollisionResponseToChannel` (`self.SpaceFour`) "ECC_GameTraceChannel3" "ECR_Ignore")
    (set `/Game/FirstPerson/Blueprints/Items/BP_BaseItem.SpaceBoxRef` (`self.SpaceFour`) _asbp_base_item)
    (`KismetSystemLibrary.PrintString` "4")))

(event `self.SpaceFive.OnComponentBeginOverlap`
  (params (OverlappedComponent :type "PrimitiveComponent Object Reference") (OtherActor :type "Actor Object Reference") (OtherComp :type "PrimitiveComponent Object Reference") (OtherBodyIndex :type Integer) (bFromSweep :type Boolean) (SweepResult :type "HitResult Structure (by ref)"))
  (bind _asbp_base_item (cast `/Game/FirstPerson/Blueprints/Items/BP_BaseItem` OtherActor))
  (if (`|EnumEquality` (`/Game/FirstPerson/Blueprints/Items/BP_BaseItem.ItemState` _asbp_base_item) "NewEnumerator2")
    (`PrimitiveComponent.SetCollisionResponseToChannel` (`self.SpaceFive`) "ECC_GameTraceChannel3" "ECR_Ignore")
    (set `/Game/FirstPerson/Blueprints/Items/BP_BaseItem.SpaceBoxRef` (`self.SpaceFive`) _asbp_base_item)
    (`KismetSystemLibrary.PrintString` "5")))

(fn `CheckOverCooked`
  (for _array_element (`self.Items`)
    (if (`|EnumEquality` (`/Game/FirstPerson/Blueprints/Items/BP_BaseItem.CookState` _array_element) "NewEnumerator4")
      (`self.PalyOverCookSound`)
      (else
        (`self.CheckOverCooked`))))
  (`KismetSystemLibrary.PrintString` "Hello"))

(fn `MultipleCook`
  (`|ExecutionSequence`
    (:`then_0`
      (if (`self.Clicked?`)
        (for _array_element (`self.Items`)
          (bind _returnvalue (`KismetSystemLibrary.K2_SetTimer` _array_element "Cooking" 2.0))
          (`self.PlayCookSound` (`KismetSystemLibrary.K2_GetTimerRemainingTimeHandle` _returnvalue)))))))

(fn `UserConstructionScript`)