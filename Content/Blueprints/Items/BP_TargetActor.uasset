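; Spawn-point actor that creates purchased items at its own transform and charges the player for them.
; SpawnItem switches on the item type (Clay, Sesame, Egg) and spawns a BP_BaseItem, setting ItemType for all but Clay, which relies on the class default.
; Each spawned item's Cost is then deducted from player 0's BP_PideciState through DecreaseMoney, with no affordability check here.
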(event `SpawnItem`
  (params (L_ItemType :type "/Game/FirstPerson/Blueprints/Enums/ItemType Enum" :default "NewEnumerator8"))
  (switch `/Game/FirstPerson/Blueprints/Enums/ItemType` L_ItemType
    (:`NewEnumerator0`
      (bind _returnvalue (`|SpawnActorFromClass` "/Game/FirstPerson/Blueprints/Items/BP_BaseItem.BP_BaseItem_C" (`self.GetTransform`) "Undefined" "MultiplyWithRoot" null "NewEnumerator0" null))
      (`/Game/FirstPerson/Blueprints/BP_PideciState.DecreaseMoney` (cast `/Game/FirstPerson/Blueprints/BP_PideciState` (`GameplayStatics.GetPlayerState` 0) :!pure true) (`/Game/FirstPerson/Blueprints/Items/BP_BaseItem.Cost` _returnvalue)))
    (:`NewEnumerator1`
      (bind _returnvalue_2 (`|SpawnActorFromClass` "/Game/FirstPerson/Blueprints/Items/BP_BaseItem.BP_BaseItem_C" (`self.GetTransform`) "Undefined" "MultiplyWithRoot" null "NewEnumerator1" null))
      (`/Game/FirstPerson/Blueprints/BP_PideciState.DecreaseMoney` (cast `/Game/FirstPerson/Blueprints/BP_PideciState` (`GameplayStatics.GetPlayerState` 0) :!pure true) (`/Game/FirstPerson/Blueprints/Items/BP_BaseItem.Cost` _returnvalue_2)))
    (:`NewEnumerator4`
      (bind _returnvalue_3 (`|SpawnActorFromClass` "/Game/FirstPerson/Blueprints/Items/BP_BaseItem.BP_BaseItem_C" (`self.GetTransform`) "Undefined" "MultiplyWithRoot" null "NewEnumerator4" null))
      (`/Game/FirstPerson/Blueprints/BP_PideciState.DecreaseMoney` (cast `/Game/FirstPerson/Blueprints/BP_PideciState` (`GameplayStatics.GetPlayerState` 0) :!pure true) (`/Game/FirstPerson/Blueprints/Items/BP_BaseItem.Cost` _returnvalue_3)))))

(fn `UserConstructionScript`)