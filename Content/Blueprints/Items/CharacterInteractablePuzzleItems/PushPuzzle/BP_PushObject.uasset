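; BP_PushObject is a pushable puzzle object that stays snapped to the surface beneath it.
; Every Tick, a debug-drawn Visibility line trace runs from the actor to its negated, scaled Z, and the actor's height is set just above the hit location.
; Speed/Direction selects the right or forward vector from a boolean, scales it by a speed input and VInterps the relative location toward that offset, without sweep.
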(event `self.ReceiveBeginPlay`)

(event `self.ReceiveTick`
  (params (DeltaSeconds :type "Float (single-precision)"))
  (bind (_returnvalue_x _returnvalue_y _returnvalue_z) (`KismetMathLibrary.BreakVector` (`self.K2_GetActorLocation`)))
  (bind (_returnvalue_x_2 _returnvalue_y_2) (`KismetMathLibrary.BreakVector` (`self.K2_GetActorLocation`)))
  (bind _outhit (`KismetSystemLibrary.LineTraceSingle` :`Start` (`self.K2_GetActorLocation`) :`End` (`KismetMathLibrary.MakeVector` _returnvalue_x _returnvalue_y (* _returnvalue_z -10.0)) :`TraceChannel` "TraceTypeQuery1" :`DrawDebugType` "ForDuration"))
  (`self.K2_SetActorLocation` (`KismetMathLibrary.MakeVector` _returnvalue_x_2 _returnvalue_y_2 (+ (.z (`.Location` (`GameplayStatics.BreakHitResult` _outhit))) 50.0))))

(fn `UserConstructionScript`)