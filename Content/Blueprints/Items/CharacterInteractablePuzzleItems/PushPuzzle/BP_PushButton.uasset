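; Pressure-plate button for the push puzzle that opens its linked Door and sinks or raises its Floor mesh via a timeline.
; Any actor entering the Box opens the door and plays the timeline, but only actors tagged PushableObject or WarriorCharacter are counted.
; When an overlap ends with the count at zero or below, a short delay precedes closing the door and reversing the timeline.
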(event `self.Box.OnComponentBeginOverlap`
  (params (OverlappedComponent :type "PrimitiveComponent Object Reference") (OtherActor :type "Actor Object Reference") (OtherComp :type "PrimitiveComponent Object Reference") (OtherBodyIndex :type Integer) (bFromSweep :type Boolean) (SweepResult :type "HitResult Structure (by ref)"))
  (`|ExecutionSequence`
    (:`then_0`
      (`/Game/Blueprints/Items/CharacterInteractablePuzzleItems/PushPuzzle/BP_PuzzleDoor.OpenDoor` (`self.Door`))
      (bind (_direction _newtrack_0) (`Timeline|PushTimeline` :!label _label)
        (:`Update`
          (`SceneComponent.K2_SetRelativeLocation` (`self.Floor`) (`KismetMathLibrary.MakeVector` 0.0 0.0 _newtrack_0) false false))))
    (:`then_1`
      (`self.IncreaseObjectCount` OtherActor))))

(event `self.Box.OnComponentEndOverlap`
  (params (OverlappedComponent :type "PrimitiveComponent Object Reference") (OtherActor :type "Actor Object Reference") (OtherComp :type "PrimitiveComponent Object Reference") (OtherBodyIndex :type Integer))
  (`|ExecutionSequence`
    (:`then_0`
      (`self.DecreaseObjectCount` OtherActor))
    (:`then_1`
      (if (<= (`self.Object`) 0)
        (`KismetSystemLibrary.Delay` 0.2)
        (`/Game/Blueprints/Items/CharacterInteractablePuzzleItems/PushPuzzle/BP_PuzzleDoor.CloseDoor` (`self.Door`))
        (goto _label :!via `Reverse`)))))

(event `self.ReceiveActorEndOverlap`
  (params (OtherActor :type "Actor Object Reference")))

(fn `DecreaseObjectCount`
  (params (OverlappedActor :type "Actor Object Reference"))
  (if (`self.ActorHasTag` OverlappedActor "PushableObject")
    (`/Engine/EditorBlueprintResources/StandardMacros.DecrementInt` (`self.Object`))
    (elif (`self.ActorHasTag` OverlappedActor "WarriorCharacter")
      (`/Engine/EditorBlueprintResources/StandardMacros.DecrementInt` (`self.Object`)))))

(fn `IncreaseObjectCount`
  (params (OverlappingActor :type "Actor Object Reference"))
  (if (`self.ActorHasTag` OverlappingActor "PushableObject")
    (`/Engine/EditorBlueprintResources/StandardMacros.IncrementInt` (`self.Object`))
    (elif (`self.ActorHasTag` OverlappingActor "WarriorCharacter")
      (`/Engine/EditorBlueprintResources/StandardMacros.IncrementInt` (`self.Object`)))))

(fn `UserConstructionScript`)