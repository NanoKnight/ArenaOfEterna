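; BP_PideciState is a state Blueprint that holds the player's money and customer pleasure values.
; It exposes simple add and subtract functions for each value, with inputs named the same as the variables they change.
; The functions apply no clamping or notifications, and the event graph and construction script are empty.
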(fn `AddPleasure`
  (params (CustomerPleasure :type Integer))
  (set `self.CustomerPleasure` (+ CustomerPleasure (`self.CustomerPleasure`))))

(fn `DecrasePleasure`
  (params (CustomerPleasure :type Integer))
  (set `self.CustomerPleasure` (- (`self.CustomerPleasure`) CustomerPleasure)))

(fn `DecreaseMoney`
  (params (Money :type Integer))
  (set `self.Money` (- (`self.Money`) Money)))

(fn `IncreaseMoney`
  (params (Money :type Integer))
  (set `self.Money` (+ Money (`self.Money`))))

(fn `UserConstructionScript`)