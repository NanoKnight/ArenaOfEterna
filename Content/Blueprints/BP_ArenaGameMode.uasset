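; BP_ArenaGameMode is an arena game mode that adds wave text UI to enemy respawning.
; On BeginPlay it creates a WB_WaveText widget and caches the level's BP_EnemySpawner.
; RespawnEnemyStart extends the parent event: in WaveMode it adds the widget to the viewport, then immediately removes it if its SecondsCounter is zero.
; Tick only calls the parent, and a debug print of ChasedEnemies is left disconnected.
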(event `self.ReceiveBeginPlay`
  (`|ExecutionSequence`
    (:`then_0`
      (`parent.ReceiveBeginPlay`)
      (bind _returnvalue (`|CreateWidget` "/Game/Blueprints/Widgetrs/WB_WaveText.WB_WaveText_C"))
      (set `self.WaveTextWB` _returnvalue)
      (bind _returnvalue_2 (`GameplayStatics.GetActorOfClass` "/Game/Blueprints/EnemySpawners/BP_EnemySpawner.BP_EnemySpawner_C"))
      (bind _asbp_enemy_spawner (cast `/Game/Blueprints/EnemySpawners/BP_EnemySpawner` _returnvalue_2))
      (set `self.EnemySpawner` _asbp_enemy_spawner))))

(event `self.ReceiveTick`
  (params (DeltaSeconds :type "Float (single-precision)"))
  (`parent.ReceiveTick` DeltaSeconds))

(event `RespawnEnemyInterface.RespawnEnemyStart`
  (bind _wavetextwb (`self.WaveTextWB`))
  (`parent.RespawnEnemyStart`)
  (if (`self.Wave Mode`)
    (`UserWidget.AddToViewport` _wavetextwb 0)
    (if (== (`/Game/Blueprints/Widgetrs/WB_WaveText.secondsCounter` _wavetextwb) 0)
      (`Widget.RemoveFromParent` _wavetextwb))))

(fn `UserConstructionScript`
  (`parent.UserConstructionScript`))