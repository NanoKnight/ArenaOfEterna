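; Demon enemy Blueprint that feeds Motion Warping targets from its CombatTarget.
; Tick updates the RotationTarget warp point through GetRotationWarpTarget, or removes the rotation and translation targets when CombatTarget is invalid.
; A SetWarpTarget event registers the target's full transform as the CombatTarget warp target.
; The TranslationTarget update via GetTranslationWarpTarget is disconnected and never runs.
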(event `self.ReceiveTick`
  (params (DeltaSeconds :type "Float (single-precision)"))
  (bind _motionwarping (`self.MotionWarping`))
  (bind _combattarget (`self.CombatTarget`)
    (:`then`
      (bind _returnvalue (`self.GetRotationWarpTarget` _combattarget))
      (`MotionWarpingComponent.AddOrUpdateWarpTargetFromLocation` (`self.MotionWarping`) "RotationTarget" _returnvalue))
    (:`else`
      (`MotionWarpingComponent.RemoveWarpTarget` _motionwarping "TranslationTarget")
      (`MotionWarpingComponent.RemoveWarpTarget` _motionwarping "RotationTarget"))))

(event `SetWarpTarget`
  (bind _combattarget (`self.CombatTarget`)
    (:`then`
      (`MotionWarpingComponent.AddOrUpdateWarpTargetFromTransform` (`self.MotionWarping`) "CombatTarget" (`self.GetTransform` _combattarget)))
    (:`else`)))

(fn `UserConstructionScript`)