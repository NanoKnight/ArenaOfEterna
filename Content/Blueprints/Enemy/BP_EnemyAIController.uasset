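; Enemy AI controller that reacts to perception updates and writes the enemy's Patrolling or Chasing state to the Blackboard.
; On each update it checks every actor for sight, hearing and damage through CanSense, which matches stimuli to an enum-selected sense class.
; Sight switches the state to Chasing, while hearing and damage only print debug text.
; The behavior tree launch and initial Patrolling call are disconnected, so neither runs.
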(event `self.ReceivePossess`
  (params (PossessedPawn :type "Pawn Object Reference")))

(event `self.ReceiveBeginPlay`)

(event `self.AIPerception.OnPerceptionUpdated`
  (params (UpdatedActors :type "Array of Actor Object Reference (by ref)"))
  (for _array_element UpdatedActors
    (`|ExecutionSequence`
      (:`then_0`
        (bind _sensed (`self.CanSense` _array_element "NewEnumerator1"))
        (if _sensed
          (`KismetSystemLibrary.PrintString` "Sight")
          (`self.SetChasing`)))
      (:`then_1`
        (bind _sensed_2 (`self.CanSense` _array_element "NewEnumerator2"))
        (if _sensed_2
          (`KismetSystemLibrary.PrintString` "Heard")))
      (:`then_2`
        (bind _sensed_3 (`self.CanSense` _array_element "NewEnumerator3"))
        (if _sensed_3
          (`KismetSystemLibrary.PrintString` "Damaged"))))))

(fn `CanSense`
  (params (Actor :type "Actor Object Reference") (AISense :type "/Game/Blueprints/Enums/AISense Enum" :default "NewEnumerator0"))
  (returns (Sensed :type Boolean) (Stimulus :type "AIStimulus Structure"))
  (bind _info (`AIPerceptionComponent.GetActorsPerception` (`self.AIPerception`) Actor))
  (for _array_element (`.LastSensedStimuli` (break `ActorPerceptionBlueprintInfo` _info))
    (bind _returnvalue (`AIPerceptionSystem.GetSenseClassForStimulus` _array_element))
    (if (== _returnvalue (select `/Game/Blueprints/Enums/AISense` AISense :`NewEnumerator1` "/Script/AIModule.AISense_Sight" :`NewEnumerator2` "/Script/AIModule.AISense_Hearing" :`NewEnumerator3` "/Script/AIModule.AISense_Damage" :!type "Object Class Reference"))
      (return (`.bSuccessfullySensed` (break `AIStimulus` _array_element)) _array_element))))

(fn `SetChasing`
  (`BlackboardComponent.SetValueAsEnum` (`self.Blackboard`) (`self.State`) (enumliteral `EEnemyState` "EES_Chasing")))

(fn `SetPatrolling`
  (`BlackboardComponent.SetValueAsEnum` (`self.Blackboard`) (`self.State`) (enumliteral `EEnemyState` "EES_Patrolling")))

(fn `UserConstructionScript`)