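; Demon enemy character that prepares motion-warp targets against its combat target and sets movement speed by AI state.
; Each tick, it updates rotation and translation warp targets while the target is within close range, otherwise removing both.
; A separate SetWarpTarget event registers the target's full transform as a warp target.
; SetState selects walk speed for patrolling, run speed for chasing and zero otherwise; GetPatrolRoute exposes its route.
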(event `self.ReceiveTick`
  (params (DeltaSeconds :type "Float (single-precision)"))
  (bind _motionwarping (`self.MotionWarping`))
  (bind _combattarget (`self.CombatTarget`)
    (:`then`
      (if (<= (`self.GetDistanceTo` _combattarget self) 350.0)
        (bind _returnvalue (`self.GetRotationWarpTarget` _combattarget))
        (`MotionWarpingComponent.AddOrUpdateWarpTargetFromLocation` (`self.MotionWarping`) "RotationTarget" _returnvalue)
        ;[1 1 1] FOR WAR LOCATION
        (bind _returnvalue_2 (`self.GetTranslationWarpTarget` _combattarget))
        (`MotionWarpingComponent.AddOrUpdateWarpTargetFromLocation` (`self.MotionWarping`) "TranslationTarget" _returnvalue_2)
        (else
          (`MotionWarpingComponent.RemoveWarpTarget` _motionwarping "TranslationTarget" :!label _label)
          (`MotionWarpingComponent.RemoveWarpTarget` _motionwarping "RotationTarget"))))
    (:`else`
      (goto _label))))

(event `SetWarpTarget`
  (bind _combattarget (`self.CombatTarget`)
    (:`then`
      (`MotionWarpingComponent.AddOrUpdateWarpTargetFromTransform` (`self.MotionWarping`) "CombatTarget" (`self.GetTransform` _combattarget)))
    (:`else`)))

(fn `GetPatrolRoute`
  (returns (PatrolRoute :type "/Game/Blueprints/Enemy/BehaviorTree/BP_PatrolRoute Object Reference"))
  (return (`self.PatrolRoute`)))

(fn `SetState`
  (params (EnemyState :type "EEnemyState Enum" :default "EES_NoState"))
  (set `CharacterMovementComponent.MaxWalkSpeed` (select `EEnemyState` EnemyState :`EES_Patrolling` (`self.WalkSpeed`) :`EES_Chasing` (`self.RunSpeed`) :!type "Float (double-precision)") (`self.CharacterMovement`))
  (return))

(fn `UserConstructionScript`)