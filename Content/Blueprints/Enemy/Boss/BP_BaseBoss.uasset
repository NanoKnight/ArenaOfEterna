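; Base boss enemy Blueprint that keeps Motion Warping targets aligned with its current CombatTarget.
; Each tick it feeds locations from GetTranslationWarpTarget and GetRotationWarpTarget into separate translation and rotation warp targets, removing both when CombatTarget is invalid.
; A separate SetWarpTarget event snapshots the target's full transform into a CombatTarget warp target, which Tick never clears.
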(event `self.ReceiveBeginPlay`
  (`parent.ReceiveBeginPlay`))

(event `SetWarpTarget`
  (bind _combattarget (`self.CombatTarget`)
    (:`then`
      (`MotionWarpingComponent.AddOrUpdateWarpTargetFromTransform` (`self.MotionWarping`) "CombatTarget" (`self.GetTransform` _combattarget)))
    (:`else`)))

(event `self.ReceiveTick`
  (params (DeltaSeconds :type "Float (single-precision)"))
  (bind _motionwarping (`self.MotionWarping`))
  (`parent.ReceiveTick` DeltaSeconds)
  (bind _combattarget (`self.CombatTarget`)
    (:`then`
      (bind _returnvalue (`self.GetTranslationWarpTarget` _combattarget))
      (`MotionWarpingComponent.AddOrUpdateWarpTargetFromLocation` (`self.MotionWarping`) "TranslationTarget" _returnvalue)
      (bind _returnvalue_2 (`self.GetRotationWarpTarget` _combattarget))
      (`MotionWarpingComponent.AddOrUpdateWarpTargetFromLocation` (`self.MotionWarping`) "RotationTarget" _returnvalue_2))
    (:`else`
      (`MotionWarpingComponent.RemoveWarpTarget` _motionwarping "TranslationTarget")
      (`MotionWarpingComponent.RemoveWarpTarget` _motionwarping "RotationTarget"))))

(fn `UserConstructionScript`)