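; BP_TutorialActor is a trigger box that shows a tutorial popup when an actor tagged WarriorCharacter enters it.
; On overlap it creates WB_TutorialWidget from its video, title, description and media texture variables, switches to focused UI-only input and pauses the game.
; The actor destroys itself on any end overlap, without checking the tag.
; Unpausing and restoring game input are not handled in this Blueprint.
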(event `self.Box.OnComponentBeginOverlap`
  (params (OverlappedComponent :type "PrimitiveComponent Object Reference") (OtherActor :type "Actor Object Reference") (OtherComp :type "PrimitiveComponent Object Reference") (OtherBodyIndex :type Integer) (bFromSweep :type Boolean) (SweepResult :type "HitResult Structure (by ref)"))
  (if (`self.ActorHasTag` OtherActor "WarriorCharacter")
    (bind _returnvalue (`|CreateWidget` "/Game/Blueprints/Widgetrs/WB_TutorialWidget.WB_TutorialWidget_C" null "/Game/Images/TutorialIcons/TutorialVideos/video.video" (`self.Tutorial Title`) (`self.Tutorial Description`) (`self.Media Texture Value`)))
    (`WidgetBlueprintLibrary.SetInputMode_UIOnlyEx` (`GameplayStatics.GetPlayerController` 0) _returnvalue "DoNotLock" true)
    (`UserWidget.AddToViewport` _returnvalue 0)
    (`Widget.SetCursor` _returnvalue "None")
    (`Widget.SetKeyboardFocus` _returnvalue)
    (`GameplayStatics.SetGamePaused` true)))

(event `self.Box.OnComponentEndOverlap`
  (params (OverlappedComponent :type "PrimitiveComponent Object Reference") (OtherActor :type "Actor Object Reference") (OtherComp :type "PrimitiveComponent Object Reference") (OtherBodyIndex :type Integer))
  (`self.K2_DestroyActor`))

(fn `UserConstructionScript`)