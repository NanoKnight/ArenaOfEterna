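; Warrior character Blueprint that feeds Motion Warping targets from a nearby enemy and adds a few key-driven actions.
; Each tick it updates translation and rotation warp targets from CloseEnemy, or removes both when that enemy is invalid.
; F plays the Deneme montage, Z toggles slow motion through a console command, and BeginPlay assigns an outline material to OverlayMaterial.
; The Sphere overlap events are empty, and CloseEnemy is not set here.
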(event `Key|F`
  (params (Key :type "Key Structure"))
  (:`Pressed`
    (`|PlayMontage` (`self.Mesh`) "/Game/Protector/Protector/Movement/Root/deneme.deneme")))

(event `self.Sphere.OnComponentBeginOverlap`
  (params (OverlappedComponent :type "PrimitiveComponent Object Reference") (OtherActor :type "Actor Object Reference") (OtherComp :type "PrimitiveComponent Object Reference") (OtherBodyIndex :type Integer) (bFromSweep :type Boolean) (SweepResult :type "HitResult Structure (by ref)")))

(event `Key|Z`
  (params (Key :type "Key Structure"))
  (:`Pressed`
    (`/Engine/EditorBlueprintResources/StandardMacros.FlipFlop`
      (:`A`
        (`KismetSystemLibrary.ExecuteConsoleCommand` "Slomo 0.5" null))
      (:`B`
        (`KismetSystemLibrary.ExecuteConsoleCommand` "Slomo 1" null)))))

(event `self.Sphere.OnComponentEndOverlap`
  (params (OverlappedComponent :type "PrimitiveComponent Object Reference") (OtherActor :type "Actor Object Reference") (OtherComp :type "PrimitiveComponent Object Reference") (OtherBodyIndex :type Integer)))

(event `self.ReceiveBeginPlay`
  (`parent.ReceiveBeginPlay`)
  (set `self.OverlayMaterial` "/Game/Effects/Materials/Outline_Mat.Outline_Mat"))

(event `self.ReceiveTick`
  (params (DeltaSeconds :type "Float (single-precision)"))
  (bind _motionwarping (`self.MotionWarping`))
  (`parent.ReceiveTick` DeltaSeconds)
  (`|ExecutionSequence`
    (:`then_0`
      (bind _closeenemy (`self.CloseEnemy`)
        (:`then`
          (bind _returnvalue (`self.GetTranslationWarpTarget` _closeenemy))
          (`MotionWarpingComponent.AddOrUpdateWarpTargetFromLocation` (`self.MotionWarping`) "TranslationTarget" _returnvalue)
          (bind _returnvalue_2 (`self.GetRotationWarpTarget` _closeenemy))
          (`MotionWarpingComponent.AddOrUpdateWarpTargetFromLocation` (`self.MotionWarping`) "RotationTarget" _returnvalue_2))
        (:`else`
          (`MotionWarpingComponent.RemoveWarpTarget` _motionwarping "TranslationTarget")
          (`MotionWarpingComponent.RemoveWarpTarget` _motionwarping "RotationTarget"))))))

(fn `UserConstructionScript`
  (`parent.UserConstructionScript`))