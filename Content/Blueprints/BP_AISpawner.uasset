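; Spawner actor that creates waves of AI customers when BP_FirstPersonGameMode fires its respawn-enemy event.
; CustomerPleasure from BP_PideciState sets the pace: high values spawn a whole wave at once, lower ones use longer delays, and below -3 nothing spawns.
; Instant waves loop over EnemyClass, while delayed waves re-call themselves after a Delay and use hardcoded BP_BaseAI.
; Spawns are offset on Y by index, and EnemyCount grows after each wave.
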(event `self.ReceiveBeginPlay`
  (bind _asbp_first_person_game_mode (cast `/Game/FirstPerson/Blueprints/BP_FirstPersonGameMode` (`GameplayStatics.GetGameMode`)))
  (add `/Game/FirstPerson/Blueprints/BP_FirstPersonGameMode.RespawnEnemy` _asbp_first_person_game_mode (delegate `Spawn Customer`)))

(event `Spawn Customer`
  (bind _customerpleasure (`/Game/FirstPerson/Blueprints/BP_PideciState.CustomerPleasure` (cast `/Game/FirstPerson/Blueprints/BP_PideciState` (`GameplayStatics.GetPlayerState` 0) :!pure true)))
  (if (>= _customerpleasure 25)
    (`self.SpawnWithoutDelay`)
    (elif (>= _customerpleasure 21)
      (`self.SpawnWithDelay` 2.0)
      (elif (>= _customerpleasure 15)
        (`self.SpawnWithDelay` 5.0)
        (`KismetSystemLibrary.PrintString` "ananıskm")
        (elif (>= _customerpleasure 13)
          (`self.SpawnWithDelay` 7.0)
          (elif (>= _customerpleasure 10)
            (`self.SpawnWithDelay` 10.0)
            (elif (>= _customerpleasure 7)
              (`self.SpawnWithDelay` 12.0)
              (elif (>= _customerpleasure 3)
                (`self.SpawnWithDelay` 15.0)
                (elif (>= _customerpleasure 0)
                  (`self.SpawnWithDelay` 20.0)
                  (elif (>= _customerpleasure -3)
                    (`self.SpawnWithDelay` 35.0)))))))))))

(event `SpawnWithoutDelay`
  (bind (_returnvalue_location _returnvalue_rotation _returnvalue_scale) (`KismetMathLibrary.BreakTransform` (`self.GetTransform`)))
  (bind (_loc_x _loc_y _loc_z) (`KismetMathLibrary.BreakVector` (`self.Loc`)))
  (for _index (range (`self.EnemyCount`))
    (set `self.Loc` (`self.K2_GetActorLocation`))
    (`|SpawnActorFromClass` (`self.EnemyClass`) (`KismetMathLibrary.MakeTransform` (`KismetMathLibrary.MakeVector` _loc_x (* (/ (* _loc_y _index) 6.0) -1.0) _loc_z) _returnvalue_rotation _returnvalue_scale) "Undefined" "MultiplyWithRoot" null null))
  (`/Engine/EditorBlueprintResources/StandardMacros.IncrementInt` (`self.EnemyCount`)
    (:`  `
      (`KismetSystemLibrary.Delay` 1.0))))

(event `SpawnWithDelay`
  (params (Duration :type "Float (single-precision)"))
  (bind _returnvalue (`self.GetTransform`))
  (if (< (`self.CurrentEnemyCount`) (`self.EnemyCount`))
    (`/Engine/EditorBlueprintResources/StandardMacros.IncrementInt` (`self.CurrentEnemyCount`)
      (:`  `
        (`|SpawnActorFromClass` "/Game/FirstPerson/Blueprints/AI/BP_BaseAI.BP_BaseAI_C" (`KismetMathLibrary.MakeTransform` (`KismetMathLibrary.MakeVector` (.x (.location _returnvalue)) (* (/ (* (.y (.location _returnvalue)) (`self.CurrentEnemyCount`)) 6.0) -1.0) (.z (.location _returnvalue))) (.rotation _returnvalue) (.scale _returnvalue)) "Undefined" "MultiplyWithRoot" null null)
        (`KismetSystemLibrary.Delay` Duration)
        (`self.SpawnWithDelay` Duration)
        (set `self.CurrentEnemyCount` 0)))
    (elif (>= (`self.CurrentEnemyCount`) (`self.EnemyCount`))
      (`/Engine/EditorBlueprintResources/StandardMacros.IncrementInt` (`self.EnemyCount`)))))

(fn `UserConstructionScript`)