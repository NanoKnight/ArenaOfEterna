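; Preview actor that mirrors whether the player's BP_WarriorCharacters has a weapon equipped, using its own Mesh and ChildActor components.
; BeginPlay caches the player character, and Tick scans its InventoryComponent's EquippedItems every frame.
; For any Weapon-slot item, it re-attaches the ChildActor to the Mesh's Sword socket, without setting the child's class or detaching it.
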(event `self.ReceiveBeginPlay`
  (bind _asbp_warrior_characters (cast `/Game/Blueprints/BP_WarriorCharacters` (`GameplayStatics.GetPlayerCharacter` 0)))
  (set `self.As BP Warrior Characters` _asbp_warrior_characters))

(event `self.ReceiveTick`
  (params (DeltaSeconds :type "Float (single-precision)"))
  (for _array_element (`InventoryComponent.EquippedItems` (`BaseCharacter.InventoryComponent` (`self.As BP Warrior Characters`)))
    (if (`|EnumEquality` (`.EquipmentSlot` (break `InventoryStruct` _array_element)) "Weapon")
      (`SceneComponent.K2_AttachToComponent` (`self.ChildActor`) (`self.Mesh`) "Sword" "KeepRelative" "KeepRelative" "KeepRelative" true))))

(fn `UserConstructionScript`)