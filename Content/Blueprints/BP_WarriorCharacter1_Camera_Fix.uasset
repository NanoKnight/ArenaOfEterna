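; Player warrior character Blueprint that adds motion warping, an offscreen indicator widget and a pause menu to its parent class.
; Each tick it feeds translation and rotation warp targets from CloseEnemy, falling back to CloseBreakable, and removes them when neither is valid.
; Z toggles half-speed slomo, and G plays a dodge montage with a launch along world X rather than the character's facing.
; Sphere overlap handlers are empty apart from a debug print for breakables.
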(event `self.ReceiveBeginPlay`
  (`|ExecutionSequence`
    (:`then_0`
      (`parent.ReceiveBeginPlay`)
      (set `self.EnemyOutlineMaterial` "/Game/Effects/Materials/Outline_Mat1.Outline_Mat1")
      (bind _returnvalue (`|CreateWidget` "/Game/Blueprints/Widgetrs/WB_IndicatorOffscreen.WB_IndicatorOffscreen_C"))
      (`UserWidget.AddToViewport` _returnvalue 0))))

(event `self.ReceiveTick`
  (params (DeltaSeconds :type "Float (single-precision)"))
  (bind _motionwarping (`self.MotionWarping`))
  (`parent.ReceiveTick` DeltaSeconds)
  (`|ExecutionSequence`
    (:`then_0`
      (bind _closeenemy (`self.CloseEnemy`)
        (:`then`
          (bind _returnvalue (`self.GetTranslationWarpTarget` _closeenemy))
          (`MotionWarpingComponent.AddOrUpdateWarpTargetFromLocation` (`self.MotionWarping`) "TranslationTarget" _returnvalue)
          (bind _returnvalue_2 (`self.GetRotationWarpTarget` _closeenemy))
          (`MotionWarpingComponent.AddOrUpdateWarpTargetFromLocation` (`self.MotionWarping`) "RotationTarget" _returnvalue_2))
        (:`else`
          (bind _closebreakable (`self.CloseBreakable`)
            (:`then`
              (bind _returnvalue_3 (`self.GetTranslationWarpTarget` _closebreakable))
              (`MotionWarpingComponent.AddOrUpdateWarpTargetFromLocation` (`self.MotionWarping`) "TranslationTarget" _returnvalue_3)
              (bind _returnvalue_4 (`self.GetRotationWarpTarget` _closebreakable))
              (`MotionWarpingComponent.AddOrUpdateWarpTargetFromLocation` (`self.MotionWarping`) "RotationTarget" _returnvalue_4))
            (:`else`
              (`MotionWarpingComponent.RemoveWarpTarget` _motionwarping "TranslationTarget")
              (`MotionWarpingComponent.RemoveWarpTarget` _motionwarping "RotationTarget"))))))))

(event `Key|Z`
  (params (Key :type "Key Structure"))
  (:`Pressed`
    (`/Engine/EditorBlueprintResources/StandardMacros.FlipFlop`
      (:`A`
        (`KismetSystemLibrary.ExecuteConsoleCommand` "Slomo 0.5" null))
      (:`B`
        (`KismetSystemLibrary.ExecuteConsoleCommand` "Slomo 1" null)))))

(event `Key|G`
  (params (Key :type "Key Structure"))
  (:`Pressed`
    (`self.PlayAnimMontage` "/Game/Animation/AM_DodgeMontage.AM_DodgeMontage")
    (`self.LaunchCharacter` (* (`KismetMathLibrary.GetForwardVector` (struct)) 20000.0))))

(event `self.Sphere.OnComponentBeginOverlap`
  (params (OverlappedComponent :type "PrimitiveComponent Object Reference") (OtherActor :type "Actor Object Reference") (OtherComp :type "PrimitiveComponent Object Reference") (OtherBodyIndex :type Integer) (bFromSweep :type Boolean) (SweepResult :type "HitResult Structure (by ref)"))
  (cast `BreakableActor` OtherActor)
  (`KismetSystemLibrary.PrintString` "breakable"))

(event `self.Sphere.OnComponentEndOverlap`
  (params (OverlappedComponent :type "PrimitiveComponent Object Reference") (OtherActor :type "Actor Object Reference") (OtherComp :type "PrimitiveComponent Object Reference") (OtherBodyIndex :type Integer)))

(event `self.EnemyDetectionSphere.OnComponentBeginOverlap`
  (params (OverlappedComponent :type "PrimitiveComponent Object Reference") (OtherActor :type "Actor Object Reference") (OtherComp :type "PrimitiveComponent Object Reference") (OtherBodyIndex :type Integer) (bFromSweep :type Boolean) (SweepResult :type "HitResult Structure (by ref)")))

(event `self.EnemyDetectionSphere.OnComponentEndOverlap`
  (params (OverlappedComponent :type "PrimitiveComponent Object Reference") (OtherActor :type "Actor Object Reference") (OtherComp :type "PrimitiveComponent Object Reference") (OtherBodyIndex :type Integer)))

(event `InputAction|Pause`
  (params (Key :type "Key Structure"))
  (bind _returnvalue (`GameplayStatics.GetPlayerController` 0))
  (:`Pressed`
    (bind _returnvalue_2 (`|CreateWidget` "/Game/Blueprints/Widgetrs/WB_Menu.WB_Menu_C"))
    (`UserWidget.AddToViewport` _returnvalue_2 0)
    (`GameplayStatics.SetGamePaused` true)
    (`WidgetBlueprintLibrary.SetInputMode_UIOnlyEx` _returnvalue null)
    (set `PlayerController.bShowMouseCursor` true _returnvalue)))

(fn `UserConstructionScript`
  (`parent.UserConstructionScript`))